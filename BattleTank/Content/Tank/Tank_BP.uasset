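; Player-controllable tank Blueprint that binds input to driving, camera and firing, leaving the logic to its components.
; On BeginPlay it hands the turret and barrel to TankAiming and both tracks to TankMovement.
; Driving input either sets each track's throttle directly or sends movement intent through TankMovement, while Fire calls TankAiming.
; Camera input yaws an azimuth gimbal and pitches the spring arm separately, scaled by delta time.
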(event EventBeginPlay
  (Class|TankAimingComponent|Initialise (Variables|Default|GetTankAiming) (Variables|Default|GetTurret) (Variables|Default|GetBarrel))
  (Class|TankMovementComponent|Initialise (Variables|Default|GetTankMovement) (Variables|Default|GetLeft%20track) (Variables|Default|GetRight%20track)))

(event Input|ActionEvents|InputActionFire
  (params (Key :type Key%20Structure :default "AnyKey"))
  (:Pressed
    (Class|TankAimingComponent|Fire (Variables|Default|GetTankAiming))))

(event Input|AxisEvents|InputAxisAimAzimuth
  (params (AxisValue :type Float%20%28single-precision%29))
  ;[1 1 1] Camera input binding
  (Transformation|AddLocalRotation (Variables|Default|GetAzimuth%20Gimbal) (Math|Rotator|MakeRotator 0.0 0.0 (* AxisValue (Utilities|Time|GetWorldDeltaSeconds) 1e+02)) false false))

(event Input|AxisEvents|InputAxisMoveLeft
  (params (AxisValue :type Float%20%28single-precision%29))
  ;[1 1 1] Movement input binding
  (Class|TankMovementComponent|IntendMoveLeft (Variables|Default|GetTankMovement) AxisValue))

(event Input|AxisEvents|InputAxisMoveRight
  (params (AxisValue :type Float%20%28single-precision%29))
  ;[1 1 1] Movement input binding
  (Class|TankMovementComponent|IntendMoveRight (Variables|Default|GetTankMovement) AxisValue))

(event Input|AxisEvents|InputAxisMoveForwards
  (params (AxisValue :type Float%20%28single-precision%29))
  ;[1 1 1] Movement input binding
  (Class|TankMovementComponent|IntendMoveForwardsBackwards (Variables|Default|GetTankMovement) AxisValue))

(event Input|AxisEvents|InputAxisLeftTrackThrottle
  (params (AxisValue :type Float%20%28single-precision%29))
  ;[1 1 1] Movement input binding
  (Class|TankTrack|SetThrottle (Variables|Default|GetLeft%20track) AxisValue))

(event Input|AxisEvents|InputAxisRightTrackThrottle
  (params (AxisValue :type Float%20%28single-precision%29))
  ;[1 1 1] Movement input binding
  (Class|TankTrack|SetThrottle (Variables|Default|GetRight%20track) AxisValue))

(event Input|AxisEvents|InputAxisMoveBackwards
  (params (AxisValue :type Float%20%28single-precision%29))
  ;[1 1 1] Movement input binding
  (Class|TankMovementComponent|IntendMoveForwardsBackwards (Variables|Default|GetTankMovement) AxisValue))

(event Input|AxisEvents|InputAxisAimElevation
  (params (AxisValue :type Float%20%28single-precision%29))
  ;[1 1 1] Camera input binding
  (Transformation|AddLocalRotation (Variables|Default|GetSpringArm) (Math|Rotator|MakeRotator 0.0 (* AxisValue (Utilities|Time|GetWorldDeltaSeconds) 1e+02) 0.0) false false))

(fn ConstructionScript)